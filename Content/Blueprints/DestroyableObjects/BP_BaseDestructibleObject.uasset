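; BP_BaseDestructibleObject is a base destructible actor that shows its health and is destroyed when that health runs out.
; On BeginPlay it binds to the health change event of its BPHealthComp component.
; Each change sets the progress bar in its WBP_HealthIndicator widget to the current health percentage, then destroys the actor if the component reports it has died.
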(event `self.ReceiveBeginPlay`
  (add `/Game/Blueprints/HealthSystem/BP_HealthComp.OnHealthChanged` (`self.BP_HealthComp`) (delegate `OnHealthChanged_Event`)))

(event `OnHealthChanged_Event`
  (bind _bp_healthcomp (`self.BP_HealthComp`))
  (bind _aswbp_health_indicator (cast `/Game/Blueprints/WidgetBlueprints/WBP_HealthIndicator` (`WidgetComponent.GetWidget` (`self.Widget`))))
  (`ProgressBar.SetPercent` (`/Game/Blueprints/WidgetBlueprints/WBP_HealthIndicator.HealthProgressBar` _aswbp_health_indicator) (`/Game/Blueprints/HealthSystem/BP_HealthComp.HealthPercentage` _bp_healthcomp))
  (if (`/Game/Blueprints/HealthSystem/BP_HealthComp.Died` _bp_healthcomp)
    (`self.K2_DestroyActor`)))

(fn `UserConstructionScript`)