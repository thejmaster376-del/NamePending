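; Game mode for the start menu level that drives the main menu and options screens.
; On BeginPlay it shows WBP_StartMenu with the cursor and UI-only input, then toggles visibility with a lazily created, cached WBP_OptionsMenu.
; New game deletes any existing SaveSlot01 save, while continue keeps it; both open the first level and switch to game-only input.
; It also provides an event to quit the game.
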(event `NewGame?`
  ; NewGameFuctionality
  (bind _returnvalue (`GameplayStatics.DoesSaveGameExist` "SaveSlot01"))
  (if _returnvalue
    (`GameplayStatics.DeleteGameInSlot` "SaveSlot01")
    (`GameplayStatics.OpenLevel` (`self.First Level Name`))
    (`WidgetBlueprintLibrary.SetInputMode_GameOnly` (`GameplayStatics.GetPlayerController` 0))
    (else
      (`GameplayStatics.OpenLevel` (`self.First Level Name`))
      (`WidgetBlueprintLibrary.SetInputMode_GameOnly` (`GameplayStatics.GetPlayerController` 0)))))

(event `ContinueGame`
  ; ContinueGame
  (`GameplayStatics.OpenLevel` (`self.First Level Name`))
  (`WidgetBlueprintLibrary.SetInputMode_GameOnly` (`GameplayStatics.GetPlayerController` 0)))

(event `ExitGame`
  ; LeavingGame
  (`KismetSystemLibrary.QuitGame` null "Quit"))

(event `LoadTheFirstLevel`
  ; OpenFirstLevel
  (`self.NewGame?`))

(event `self.ReceiveBeginPlay`
  (bind _returnvalue (`GameplayStatics.GetPlayerController` 0))
  ; StartMenuWidget
  (bind _returnvalue_2 (`|CreateWidget` "/Game/Blueprints/WidgetBlueprints/WBP_StartMenu.WBP_StartMenu_C" (`GameplayStatics.GetPlayerController` 0)))
  (bind _output_get (set `self.WidgetMainMenu` _returnvalue_2))
  (`UserWidget.AddToViewport` _output_get 0)
  (set `PlayerController.bShowMouseCursor` true _returnvalue)
  (`WidgetBlueprintLibrary.SetInputMode_UIOnlyEx` _returnvalue null))

(event `SwitchToOptions`
  ; GoingToOptionsFromStartMenu
  (`Widget.SetVisibility` (`self.WidgetMainMenu`) "Collapsed")
  (`/Engine/EditorBlueprintResources/StandardMacros.IsValid` (`self.WidgetOptionsMenu`)
    (:`Is Valid`
      (`Widget.SetVisibility` (`self.WidgetOptionsMenu`) "Visible"))
    (:`Is Not Valid`
      (bind _returnvalue (`|CreateWidget` "/Game/Blueprints/WidgetBlueprints/WBP_OptionsMenu.WBP_OptionsMenu_C"))
      (bind _output_get (set `self.WidgetOptionsMenu` _returnvalue))
      (`UserWidget.AddToViewport` _output_get 0))))

(event `SwitchToMain`
  ; LeavingOptions
  (`Widget.SetVisibility` (`self.WidgetOptionsMenu`) "Collapsed")
  (`Widget.SetVisibility` (`self.WidgetMainMenu`) "Visible"))

(fn `UserConstructionScript`)