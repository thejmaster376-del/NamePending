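; EnemySpawner is a wave system actor that spawns queued enemy classes at its own transform.
; A looping timer spawns the first queued class and removes it from the queue.
; Adding a class also triggers an immediate spawn when no BP_EnemyBase overlaps its sphere.
; It binds to each spawned enemy's destruction and has an OnEnemyDefeated event that notifies GM_CharacterFPS.
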(event `self.ReceiveBeginPlay`
  (`KismetSystemLibrary.K2_SetTimerDelegate` (delegate `TryToSpawn`) (`self.SpawnTimer`) true))

(event `TryToSpawn`
  (`self.SpawnEnemy`))

(event `OnEnemyDefeated`
  (bind _asgm_character_fps (cast `/Game/Blueprints/Gamemodes/GM_CharacterFPS` (`GameplayStatics.GetGameMode`)))
  (`/Game/Blueprints/Gamemodes/GM_CharacterFPS.OnEnemyDefeated` _asgm_character_fps))

(fn `AddEnemyToQueue`
  (params (EnemyClass :type "/Game/CharacterAssets/BP_EnemyBase Class Reference (by ref)"))
  (`KismetArrayLibrary.Array_Add` (`self.EnemyQueue`) EnemyClass)
  (if (not (`KismetArrayLibrary.Array_IsValidIndex` (`PrimitiveComponent.GetOverlappingActors` (`self.Sphere`) "/Game/CharacterAssets/BP_EnemyBase.BP_EnemyBase_C")))
    (`self.SpawnEnemy`)))

(fn `SpawnEnemy`
  (returns (Success :type Boolean))
  (if (`KismetArrayLibrary.Array_IsValidIndex` (`self.EnemyQueue`))
    (bind _returnvalue (`|SpawnActorFromClass` (`|GetArrayItem` (`self.EnemyQueue`)) (`self.GetTransform`) "AdjustIfPossibleButAlwaysSpawn" "MultiplyWithRoot" null null))
    (add `/Game/CharacterAssets/BP_EnemyBase.On Destroyed` _returnvalue (`|CreateDelegate` :!event `OnEnemyDefeated`))
    (`KismetArrayLibrary.Array_Remove` (`self.EnemyQueue`))
    (return true)
    (else
      (return false))))

(fn `UserConstructionScript`)