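; Dialogue component that runs data-table-driven conversations through a WBP_Dialogue widget.
; Interact opens the widget with cursor and Game-and-UI input, advances it, or closes it after an end row, restoring game-only input.
; Each row supplies text, an end flag and the next row and table, so conversations chain across tables.
; Open-ended opening rows spawn option widgets that reference the component, and OptionSelected jumps to a given row.
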(event `/Game/Blueprints/Dialogue/BPI_Interact.LeaveDialogue`
  (bind _returnvalue (`GameplayStatics.GetPlayerController` 0))
  (`/Engine/EditorBlueprintResources/StandardMacros.IsValid` (`self.DialogueWidget`)
    (:`Is Valid`
      (`Widget.RemoveFromParent` (`self.DialogueWidget`) :!label _label)
      (set `self.EndDialogue` false)
      (set `self.DialogueWidget` null)
      (`WidgetBlueprintLibrary.SetInputMode_GameOnly` _returnvalue)
      (set `PlayerController.bShowMouseCursor` false _returnvalue))))

(event `OptionSelected`
  (params (RowName :type Name) (DataTable :type "DataTable Object Reference"))
  (bind _dialoguewidget (`self.DialogueWidget`))
  (bind _returnvalue (`|GetDataTableRow` DataTable RowName)
    (:`then`
      (`PanelWidget.ClearChildren` (`/Game/Blueprints/Dialogue/WBP_Dialogue.OptionsScrollBox` _dialoguewidget))
      (bind (_dialogue _row _datatable _enddialogue_) (break `/Game/Blueprints/Dialogue/Dialogue_Structure` _returnvalue))
      (`/Game/Blueprints/Dialogue/WBP_Dialogue.UpdateDialogue` _dialoguewidget _dialogue)
      (set `self.Row Name` _row)
      (set `self.Data Table` _datatable)
      (set `self.EndDialogue` _enddialogue_))))

(event `/Game/Blueprints/Dialogue/BPI_Interact.Interact`
  (params (playerRef :type "/Game/CharacterAssets/Aurora/BP_AuroraFPS Object Reference"))
  (bind _returnvalue (`GameplayStatics.GetPlayerController` 0))
  (if (`self.EndDialogue`)
    (goto _label)
    (else
      (`/Engine/EditorBlueprintResources/StandardMacros.IsValid` (`self.DialogueWidget`)
        (:`Is Valid`
          (bind _returnvalue_2 (`|GetDataTableRow` (`self.Data Table`) (`self.Row Name`))
            (:`then`
              (bind (_dialogue _row _datatable _enddialogue_) (break `/Game/Blueprints/Dialogue/Dialogue_Structure` _returnvalue_2))
              (`/Game/Blueprints/Dialogue/WBP_Dialogue.UpdateDialogue` (`self.DialogueWidget`) _dialogue)
              (set `self.Row Name` _row)
              (set `self.Data Table` _datatable)
              (set `self.EndDialogue` _enddialogue_))))
        (:`Is Not Valid`
          (bind _returnvalue_3 (`|GetDataTableRow` (`self.Data Table`) (`self.Row Name`))
            (:`then`
              (bind (_dialogue_2 _row_2 _datatable_2 _enddialogue__2 _openedendeddialogue_ _openendeddialogueoptions) (break `/Game/Blueprints/Dialogue/Dialogue_Structure` _returnvalue_3))
              (bind _returnvalue_4 (`|CreateWidget` "/Game/Blueprints/Dialogue/WBP_Dialogue.WBP_Dialogue_C" null (`KismetTextLibrary.Conv_NameToText` (`self.Name`)) _dialogue_2))
              (bind _output_get (set `self.DialogueWidget` _returnvalue_4))
              (`UserWidget.AddToViewport` _output_get 0)
              (set `self.Row Name` _row_2)
              (set `self.Data Table` _datatable_2)
              (set `self.EndDialogue` _enddialogue__2)
              (`WidgetBlueprintLibrary.SetInputMode_GameAndUIEx` _returnvalue null)
              (set `PlayerController.bShowMouseCursor` true _returnvalue)
              ; Open Ended Question?
              (if _openedendeddialogue_
                (for _array_element _openendeddialogueoptions
                  (bind (_optionname _row_3 _datatable_3) (break `/Game/Blueprints/Dialogue/OptionsDialogue_Structure` _array_element))
                  (bind _returnvalue_5 (`|CreateWidget` "/Game/Blueprints/Dialogue/WBP_DialogueOptions.WBP_DialogueOptions_C" null (`KismetTextLibrary.Conv_NameToText` _optionname) self _row_3 _datatable_3))
                  (`PanelWidget.AddChild` (`/Game/Blueprints/Dialogue/WBP_Dialogue.OptionsScrollBox` (`self.DialogueWidget`)) _returnvalue_5))))))))))