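; BP_HealthComp is a health component that tracks its owner's health as it takes damage.
; On BeginPlay it binds to the owner's OnTakeAnyDamage, truncates incoming damage to an integer and clamps CurrentHealth between zero and MaxHealth.
; It then sends interface messages to the owner for damage taken, UI updates and death at zero health, leaving the reactions to the owner.
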(event `self.ReceiveBeginPlay`
  ; Taking Dmg
  (add `Actor.OnTakeAnyDamage` (`self.GetOwner`) (delegate `TakeDamage`)))

(event `TakeDamage`
  (params (DamagedActor :type "Actor Object Reference") (Damage :type "Float (single-precision)") (DamageType :type "DamageType Object Reference") (InstigatedBy :type "Controller Object Reference") (DamageCauser :type "Actor Object Reference"))
  ; Taking Dmg
  (`self.CalculateDamage` (`KismetMathLibrary.FTrunc` Damage))
  (message `/Game/Blueprints/HealthSystem/BPI_HealthComp.HealthCompNotify_TookDamage` (`self.GetOwner`) DamageCauser)
  (`self.RequestUpdateUI`)
  (`self.CheckDeath`))

(event `CalculateDamage`
  (params (Damage :type Integer))
  ; Calcs dmg, makes sure its not negative, and not above max health
  (set `self.CurrentHealth` (`KismetMathLibrary.Clamp` (- (`self.CurrentHealth`) Damage) 0 (`self.MaxHealth`))))

(event `RequestUpdateUI`
  ; UpdatesUI
  (message `/Game/Blueprints/HealthSystem/BPI_HealthComp.HealthCompNotify_UpdateUI` (`self.GetOwner`) (`self.CurrentHealth`)))

(event `CheckDeath`
  ; Checks If Dead
  (if (<= (`self.CurrentHealth`) 0)
    (message `/Game/Blueprints/HealthSystem/BPI_HealthComp.HealthCompNotify_Dead` (`self.GetOwner`))))